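; BP_BasePickupItem is a base networked pickup item with a physics-simulated mesh that players can grab.
; The server interact event passes the item to the player's grab call, disables physics and collision, and sets PickedUp.
; Server-set ItemInfo replicates the mesh to clients through its OnRep.
; OnThrown only clears PickedUp and prints; physics-restore logic is disconnected, and OnRep_PickedUp does nothing.
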(event `self.ReceiveBeginPlay`
  (`PrimitiveComponent.SetSimulatePhysics` (`self.Mesh`) true))

(event `SERVER_SetItemInfo`
  (params (ItemInfo :type "/Game/_Assets/Blueprints/Items/S_PickupItemInfo Structure"))
  ; Called from server so that when item drops, correct meshed is assigned across clients
  (set `self.ItemInfo` ItemInfo))

(event `self.SERVER_OnInteract`
  (params (Player :type "/Game/FirstPerson/Blueprints/BP_FirstPersonCharacter Object Reference"))
  (bind _mesh (`self.Mesh`))
  (if (not (`self.PickedUp`))
    (`/Game/FirstPerson/Blueprints/BP_FirstPersonCharacter.SERVER_GrabItem` Player self)
    (`PrimitiveComponent.SetSimulatePhysics` _mesh false)
    (`PrimitiveComponent.SetCollisionEnabled` _mesh "NoCollision")
    (set `self.PickedUp` true)))

(event `/Game/_Assets/Blueprints/Items/BPI_PickupItem.OnThrown`
  (set `self.PickedUp` false)
  (`KismetSystemLibrary.PrintString` "Server on thrown"))

(fn `OnRep_ItemInfo`
  (bind _iteminfo_itemmesh (break `/Game/_Assets/Blueprints/Items/S_PickupItemInfo` (`self.ItemInfo`)))
  (`StaticMeshComponent.SetStaticMesh` (`self.Mesh`) _iteminfo_itemmesh))

(fn `OnRep_PickedUp`)

(fn `UserConstructionScript`
  (`StaticMeshComponent.SetStaticMesh` (`self.Mesh`) (`self.MeshToUse`)))