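; BP_Note is a hidden world-text note that the player reveals with a red flashlight, with text, color and size set at construction.
; BeginPlay creates a dynamic text material at zero opacity.
; While the player overlaps SphereCheck, a looping timer raises an interpolated opacity whenever right click is held.
; That opacity reaches the material only when the bulb is red and a camera dot-product test confirms the note is centered in view.
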(event `self.ReceiveBeginPlay`
  (bind _returnvalue (`GameplayStatics.GetPlayerPawn` 0))
  (`KismetSystemLibrary.Delay` 1.0)
  (`KismetSystemLibrary.PrintString` (`KismetSystemLibrary.GetDisplayName` _returnvalue))
  (bind _asbp_first_person_character (cast `/Game/FirstPerson/Blueprints/BP_FirstPersonCharacter` _returnvalue))
  (set `self.PlayerRef` _asbp_first_person_character)
  (set `self.Flashlight_Ref` (`/Game/FirstPerson/Blueprints/BP_FirstPersonCharacter.FlashlightRef` _asbp_first_person_character))
  (bind _returnvalue_2 (`PrimitiveComponent.CreateDynamicMaterialInstance` (`self.TextRender`) 0 "/Game/DefaultTextMaterialOpaque_Inst.DefaultTextMaterialOpaque_Inst" "Base Color"))
  (set `self.DynamicMat` _returnvalue_2)
  (`MaterialInstanceDynamic.SetScalarParameterValue` (`self.DynamicMat`) "OpacityPower" 0.0))

(event `self.SphereCheck.OnComponentBeginOverlap`
  (params (OverlappedComponent :type "PrimitiveComponent Object Reference") (OtherActor :type "Actor Object Reference") (OtherComp :type "PrimitiveComponent Object Reference") (OtherBodyIndex :type Integer) (bFromSweep :type Boolean) (SweepResult :type "HitResult Structure (by ref)"))
  ; is player overlapping and holding down right click, check and reveal text every 2 seconds
  (cast `/Game/FirstPerson/Blueprints/BP_FirstPersonCharacter` OtherActor)
  (bind _returnvalue (`KismetSystemLibrary.K2_SetTimerDelegate` (delegate `CheckLight`) 0.2 true))
  (set `self.SaveTimer` _returnvalue))

(event `CheckLight`
  (bind _playerref (`self.PlayerRef`))
  ; is player overlapping and holding down right click, check and reveal text every 2 seconds
  (`/Engine/EditorBlueprintResources/StandardMacros.IsValid` _playerref
    (:`Is Valid`
      (if (`/Game/FirstPerson/Blueprints/BP_FirstPersonCharacter.RightClickHeld` _playerref)
        (bind _output_get (set `self.CurrentOpacity` (`KismetMathLibrary.FInterpTo` (`self.CurrentOpacity`) 1.0 (`GameplayStatics.GetWorldDeltaSeconds`) 5.0)))
        (`self.ShouldReveal` _output_get)))))

(event `ShouldReveal`
  (params (Opacity :type "Float (double-precision)"))
  (bind _returnvalue (`GameplayStatics.GetPlayerCameraManager` 0))
  (bind (_returnvalue_r _returnvalue_g _returnvalue_b) (break `LinearColor` (`LightComponentBase.GetLightColor` (`/Game/Blueprints/SM_Flashlight.BulbLight` (`self.Flashlight_Ref`)))))
  ; If stuff on the left is true change the opacity of the text
  (if (and (>= _returnvalue_r 0.8) (< _returnvalue_g 0.2) (< _returnvalue_b 0.2) (> (`KismetMathLibrary.Dot_VectorVector` (`KismetMathLibrary.Normal` (- (`self.K2_GetActorLocation`) (`self.K2_GetActorLocation` _returnvalue))) (`self.GetActorForwardVector` _returnvalue)) 0.95))
    (`MaterialInstanceDynamic.SetScalarParameterValue` (`self.DynamicMat`) "OpacityPower" Opacity)))

(event `self.SphereCheck.OnComponentEndOverlap`
  (params (OverlappedComponent :type "PrimitiveComponent Object Reference") (OtherActor :type "Actor Object Reference") (OtherComp :type "PrimitiveComponent Object Reference") (OtherBodyIndex :type Integer))
  (`KismetSystemLibrary.K2_ClearAndInvalidateTimerHandle` (`self.SaveTimer`)))

(fn `UserConstructionScript`
  (bind _textrender (`self.TextRender`))
  (`TextRenderComponent.K2_SetText` _textrender (`self.TextSet`))
  (`TextRenderComponent.SetTextRenderColor` _textrender (`self.TextColor`))
  (`TextRenderComponent.SetWorldSize` _textrender (`self.TextSize`)))