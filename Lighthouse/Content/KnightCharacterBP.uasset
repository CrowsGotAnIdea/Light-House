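; KnightCharacterBP is a knight character Blueprint holding prototype turret detection logic that only prints debug messages, with no firing.
; DetectionSphere overlaps with BP_FirstPersonCharacter store the target and toggle TurretActive.
; StartTurretLoop is a Delay-based recursive event that repeats while TurretActive is true.
; Begin overlap clears TurretActive right after starting the loop, so the delayed check fails and never repeats.
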(event `self.DetectionSphere.OnComponentBeginOverlap`
  (params (OverlappedComponent :type "PrimitiveComponent Object Reference") (OtherActor :type "Actor Object Reference") (OtherComp :type "PrimitiveComponent Object Reference") (OtherBodyIndex :type Integer) (bFromSweep :type Boolean) (SweepResult :type "HitResult Structure (by ref)"))
  (bind _asbp_first_person_character (cast `/Game/FirstPerson/Blueprints/BP_FirstPersonCharacter` OtherActor))
  (set `self.TargetPlayer` _asbp_first_person_character)
  (set `self.TurretActive` true)
  (`KismetSystemLibrary.PrintString` "Player Detected")
  (`self.StartTurretLoop`)
  (set `self.TurretActive` false))

(event `StartTurretLoop`
  (`KismetSystemLibrary.Delay` (`self.FireDelay`))
  (if (`self.TurretActive`)
    (`KismetSystemLibrary.PrintString` "Turret Checking")
    (`self.StartTurretLoop`)))

(event `self.DetectionSphere.OnComponentEndOverlap`
  (params (OverlappedComponent :type "PrimitiveComponent Object Reference") (OtherActor :type "Actor Object Reference") (OtherComp :type "PrimitiveComponent Object Reference") (OtherBodyIndex :type Integer))
  (cast `/Game/FirstPerson/Blueprints/BP_FirstPersonCharacter` OtherActor)
  (set `self.TurretActive` false)
  (`KismetSystemLibrary.PrintString` "PLAYER LEFT"))

(fn `UserConstructionScript`)